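; Player character Blueprint for a 2D Paper2D side-view game, handling movement, jumping, rolling, a four-step attack cycle, damage and death.
; Tick picks Idle, Run or Death flipbooks from state flags and velocity, and flips control rotation to face horizontal movement.
; Actions lock their state for the flipbook's length using delays, with attacks and hits also disabling input.
; Rolling blocks damage, and hits reuse the Hanging flipbook.
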(event Custom|UpdateAnimation
  ;[1 1 1] Update Animation Event
  (if (> (Variables|Default|GetHealth) 0.0)
    (if (not (Variables|Default|GetIsAttacking))
      (if (not (Variables|Default|GetBeingAttacked))
        (if (not (Variables|Default|GetIsRolling))
          (if (not (Variables|Default|GetIsJumping))
            (if (Variables|Default|GetIsRunning)
              (CallFunction|FlipbookFunction "NewEnumerator2")
              (else
                (CallFunction|FlipbookFunction (select (> (Math|Vector|VectorLength (Transformation|GetVelocity)) 0.0) "NewEnumerator2" "NewEnumerator0"))))))))
    (else
      (CallFunction|FlipbookFunction "NewEnumerator5")
      (Pawn|Components|CharacterMovement|DisableMovement (Variables|Character|GetCharacterMovement))
      (Utilities|FlowControl|Delay (Class|PaperFlipbookComponent|GetFlipbookLength (Variables|Default|GetSprite)))
      (Audio|Components|Audio|Stop (Variables|Default|GetSprite)))))

(event Custom|UpdateControlRotation
  ;[1 1 1] Update Control Rotation Event
  (Utilities|IsValid (Pawn|GetController)
    (:Is%20Valid
      (Math|Float|CompareFloat (.X (Math|Vector|BreakVector (Variables|/Script/Engine.MovementComponent|GetVelocity (Variables|Character|GetCharacterMovement)))) 0.0
        (:>
          (Pawn|SetControlRotation (Pawn|GetController) (Math|Rotator|MakeRotator 0.0 0.0 0.0)))
        (:<
          (Pawn|SetControlRotation (Pawn|GetController) (Math|Rotator|MakeRotator 0.0 0.0 1.8e+02)))))))

(event Game|Damage|EventAnyDamage
  (params (Damage :type Float%20%28single-precision%29) (DamageType :type Damage%20Type%20Object%20Reference) (InstigatedBy :type Controller%20Object%20Reference) (DamageCauser :type Actor%20Object%20Reference))
  ;[1 1 1] Take Damage
  (if (not (Variables|Default|GetIsDead))
    (if (not (Variables|Default|GetIsRolling))
      (if (not (<= (Variables|Default|GetHealth) 0.0))
        (Variables|Default|SetHealth (- (Variables|Default|GetHealth) Damage))
        (Variables|Default|SetBeingAttacked true)
        (Input|DisableInput 0)
        (CallFunction|FlipbookFunction "NewEnumerator3")
        (Utilities|FlowControl|Delay (Class|PaperFlipbookComponent|GetFlipbookLength (Variables|Default|GetSprite)))
        (Variables|Default|SetBeingAttacked false)
        (Input|EnableInput 0)))))

(event EventTick
  (params (DeltaSeconds :type Float%20%28single-precision%29))
  (CallFunction|UpdateAnimation)
  (CallFunction|UpdateControlRotation))

(event Input|ActionEvents|InputActionJump
  (params (Key :type Key%20Structure))
  ;[1 1 1] Jumping
  (:Pressed
    (if (not (Variables|Default|GetIsDead))
      (Character|Jump)
      (Variables|Default|SetIsJumping true)
      (Sprite|SetFlipbook (Variables|Default|GetSprite) (Variables|Default|GetJump_FB))
      (Utilities|FlowControl|Delay (Class|PaperFlipbookComponent|GetFlipbookLength (Variables|Default|GetSprite)))
      (Variables|Default|SetIsJumping false)))
  (:Released
    (if (not (Variables|Default|GetIsDead))
      (Character|StopJumping)
      (CallFunction|UpdateAnimation))))

(event Input|ActionEvents|InputActionRoll
  (params (Key :type Key%20Structure))
  ;[1 1 1] Rolling Stuff
  (:Pressed
    (if (not (Variables|Default|GetIsDead))
      (if (not (Variables|Default|GetIsRolling))
        (Variables|Default|SetIsRolling true)
        (Sprite|SetFlipbook (Variables|Default|GetSprite) (Variables|Default|GetRoll_FB))
        (Utilities|FlowControl|Delay (Class|PaperFlipbookComponent|GetFlipbookLength (Variables|Default|GetSprite)))
        (Variables|Default|SetIsRolling false)))))

(event Input|ActionEvents|InputActionAttack
  (params (Key :type Key%20Structure))
  (:Pressed
    (if (not (Variables|Default|GetIsDead))
      (if (not (Variables|Default|GetIsAttacking))
        (Variables|Default|SetIsAttacking true)
        (if (== (Variables|Default|GetAttackState) 1.0)
          (Sprite|SetFlipbook (Variables|Default|GetSprite) "/Game/Player/Flipbooks/Attacks/Attack_1/Player_Attack_1_FB.Player_Attack_1_FB")
          (Input|DisableInput 0)
          (Utilities|FlowControl|Delay (Class|PaperFlipbookComponent|GetFlipbookLength (Variables|Default|GetSprite)))
          (Input|EnableInput 0)
          (Variables|Default|SetAttackState 2.0)
          (Variables|Default|SetIsAttacking false)
          (elif (== (Variables|Default|GetAttackState) 2.0)
            (Sprite|SetFlipbook (Variables|Default|GetSprite) "/Game/Player/Flipbooks/Attacks/Attack_2/Player_Attack_2_FB.Player_Attack_2_FB")
            (Input|DisableInput 0)
            (Utilities|FlowControl|Delay (Class|PaperFlipbookComponent|GetFlipbookLength (Variables|Default|GetSprite)))
            (Input|EnableInput 0)
            (Variables|Default|SetAttackState 3.0)
            (Variables|Default|SetIsAttacking false)
            (elif (== (Variables|Default|GetAttackState) 3.0)
              (Sprite|SetFlipbook (Variables|Default|GetSprite) "/Game/Player/Flipbooks/Attacks/Attack_3/Player_Attack_3_FB.Player_Attack_3_FB")
              (Input|DisableInput 0)
              (Utilities|FlowControl|Delay (Class|PaperFlipbookComponent|GetFlipbookLength (Variables|Default|GetSprite)))
              (Input|EnableInput 0)
              (Variables|Default|SetAttackState 4.0)
              (Variables|Default|SetIsAttacking false)
              (elif (== (Variables|Default|GetAttackState) 4.0)
                (Sprite|SetFlipbook (Variables|Default|GetSprite) "/Game/Player/Flipbooks/Attacks/Attack_4/Player_Attack_4_FB.Player_Attack_4_FB")
                (Input|DisableInput 0)
                (Utilities|FlowControl|Delay (Class|PaperFlipbookComponent|GetFlipbookLength (Variables|Default|GetSprite)))
                (Input|EnableInput 0)
                (Variables|Default|SetAttackState 1.0)
                (Variables|Default|SetIsAttacking false)))))))))

(event Input|AxisEvents|InputAxisMoveRight
  (params (AxisValue :type Float%20%28single-precision%29))
  ;[1 1 1] Moving
  (if (not (Variables|Default|GetIsDead))
    (Pawn|Input|AddMovementInput "1.000000,0.000000,0.000000" AxisValue false)))

(fn ConstructionScript)

(fn FlipbookFunction
  (params (Current_State :type Animation_States%20Enum :default "NewEnumerator0"))
  (Variables|Default|SetAnim_States Current_State)
  (Sprite|SetFlipbook (Variables|Default|GetSprite) (Utilities|Select :Index (Variables|Default|GetAnim_States) :NewEnumerator0 (Variables|Default|GetIdle_FB) :NewEnumerator1 (Variables|Default|GetCrouch_Idle_FB) :NewEnumerator2 (Variables|Default|GetRun_FB) :NewEnumerator3 (Variables|Default|GetHanging_FB) :NewEnumerator4 (Variables|Default|GetClimb_FB) :NewEnumerator5 (Variables|Default|GetDeath_FB)))
  (return))

(fn OnRepAttackState)